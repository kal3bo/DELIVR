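; Player-controlled drone pawn, flown with Oculus controllers or keyboard, with an adjustable-length cable.
; Tick applies axis input as swept local movement and yaw, feeds delayed speed and height readings to the Drone_HUD widget, and shows a proximity warning from a sphere trace.
; SpeedUp input briefly multiplies acceleration, followed by a cooldown.
; Cable inputs grow or shrink the cable within limits checked on Tick; its overlap handler only prints debug text.
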(event `self.ReceiveTick`
  (params (DeltaSeconds :type "Float (single-precision)"))
  (bind _returnvalue (`SceneComponent.K2_GetComponentLocation` (`self.Sphere`)))
  (`|ExecutionSequence`
    (:`then_0`
      ;[1 0 0.09968] Control Input For Movement
      (`self.K2_AddActorLocalOffset` (`KismetMathLibrary.MakeVector` (* (`self.GetInputAxisValue`) (`self.Acceleration`)) (* (`self.GetInputAxisValue`) (`self.Acceleration`)) (+ (* (`self.GetInputAxisValue`) 10.0) (* (`self.GetInputAxisValue`) 10.0))) true) ; Sweep plane forwards
    )
    (:`then_1`
      ;;[1 0.8727 0] Rotate drone with Oculus (R) thumbstick X and Left & Right on the keyboard.
      (`self.K2_AddActorLocalRotation` (`KismetMathLibrary.MakeRotator` 0.0 0.0 (* (`self.GetInputAxisValue`) 1.0))))
    (:`then_2`
      ;[1 0 0.6238] Setting the Speed: Casting into the Drone Widget
      ;;[0.4583 0.4583 0.4583] Printing the speed in a way is readeable (slower)
      (`KismetSystemLibrary.Delay` 0.1)
      ;;[1 1 1] Casting and changing the parameter SPEED
      (bind _asdrone_hud (cast `/Game/Widgets/Drone_HUD` (`WidgetComponent.GetUserWidgetObject` (`self.HUD_Widget`))))
      (`/Game/Widgets/Drone_HUD.Set_Speed` _asdrone_hud (`KismetMathLibrary.VSize` (`SceneComponent.GetComponentVelocity` (`self.Speed_Sphere`)))))
    (:`then_3`
      ;[1 0.3021 0.3021] Setting the Height: Casing into the Drone widget
      (`KismetSystemLibrary.Delay` 0.1)
      (bind _asdrone_hud_2 (cast `/Game/Widgets/Drone_HUD` (`WidgetComponent.GetUserWidgetObject` (`self.HUD_Widget`))))
      (`/Game/Widgets/Drone_HUD.Set_Height` _asdrone_hud_2 (.z (`self.K2_GetActorLocation`))))
    (:`then_4`
      ;[0 0 0] Collide System: If the drone is about to collide, set the Warning Widget visible
      (bind (_outhit _returnvalue_2) (`KismetSystemLibrary.SphereTraceSingle` _returnvalue _returnvalue 300.0 "TraceTypeQuery2"))
      (if _returnvalue_2
        (`SceneComponent.SetHiddenInGame` (`self.Warning_Widget`) false false)
        (else
          (`SceneComponent.SetHiddenInGame` (`self.Warning_Widget`) true false))))
    (:`then_5`
      (`|ExecutionSequence`
        (:`then_0`
          ;[1 0.1002 0.405] Check if the cable's length is to big. If so, disable cable growth function.
          (if (>= (`CableComponent.CableLength` (`self.Cable`)) 1000.0)
            (set `self.cableAvailableDown` false)
            (else
              (set `self.cableAvailableDown` true))))
        (:`then_1`
          ;[1 0.1002 0.405] Check if the cable's length is to small. If so, disable cable growth function.
          (if (<= (`CableComponent.CableLength` (`self.Cable`)) 150.0)
            (set `self.cableAvailableUp` false)
            (else
              (set `self.cableAvailableUp` true))))))))

(event `InputAxis|SpeedUp`
  (params (AxisValue :type "Float (single-precision)"))
  ;[0.1306 0.3125 0.1783] Speed Up when player presses the left thumbstick on the Oculus controller or Space on keyboard. Acceleration increases for 3 seconds and has to rest 5 seconds to speedup again.
  (if (and (== AxisValue 1.0) (not (`self.isSpeedUpOn`)))
    (set `self.isSpeedUpOn` true)
    (`/Engine/EditorBlueprintResources/StandardMacros.DoOnce` false :!label _label
      (:`Completed`
        (set `self.Acceleration` (* (`self.Acceleration`) 1.5))
        (`KismetSystemLibrary.Delay` 3.0)
        (set `self.Acceleration` (/ (`self.Acceleration`) 1.5))
        (`KismetSystemLibrary.Delay` 5.0)
        (set `self.isSpeedUpOn` false)))
    (else
      (goto _label :!via `Reset`))))

(event `InputAxis|CableDown`
  (params (AxisValue :type "Float (single-precision)"))
  (bind _cable (`self.Cable`))
  ;[0.1864 0.7469 1] Make the cable grow function.
  (if (and (== AxisValue 1.0) (`self.cableAvailableDown`))
    (set `CableComponent.CableLength` (+ (`CableComponent.CableLength` _cable) 3.0) _cable)))

(event `InputAxis|CableUp`
  (params (AxisValue :type "Float (single-precision)"))
  (bind _cable (`self.Cable`))
  ;[0.1864 0.7469 1] Make the cable shrink function.
  (if (and (== AxisValue 1.0) (`self.cableAvailableUp`))
    (set `CableComponent.CableLength` (- (`CableComponent.CableLength` _cable) 3.0) _cable)))

(event `self.Cable.OnComponentBeginOverlap`
  (params (OverlappedComponent :type "PrimitiveComponent Object Reference") (OtherActor :type "Actor Object Reference") (OtherComp :type "PrimitiveComponent Object Reference") (OtherBodyIndex :type Integer) (bFromSweep :type Boolean) (SweepResult :type "HitResult Structure (by ref)"))
  (if (`self.ActorHasTag` OtherActor "None")
    (`KismetSystemLibrary.PrintString` "Hello")))

(fn `UserConstructionScript`
  (`parent.UserConstructionScript`))